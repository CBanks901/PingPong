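; Pong ball that drives bouncing, scoring and match end for one- and two-player levels.
; Overlaps reverse its physics velocity off paddles and boundaries, adding random X deflection on paddles; goals recenter it and update tagged score text.
; A score above 11 sets GameOver, which Tick uses to stop the ball, show win text and reload the level.
; The presence of BP_PaddleLeft selects two-player messages and level.
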(event EventBeginPlay
  (Physics|SetPhysicsLinearVelocity "0,1500.000000, 0" false "None"))

(event EventActorBeginOverlap
  (params (OtherActor :type Actor%20Object%20Reference))
  ;[1 1 1] Player Collsion Detection System
  (bind _asbp_paddle_pawn_right (Utilities|Casting|CastToBP_Paddle_Pawn_Right OtherActor)
    (:then
      (bind _returnvalue (Physics|GetPhysicsLinearVelocity _asbp_paddle_pawn_right "None"))
      (bind _returnvalue_2 (Physics|GetPhysicsLinearVelocity "None"))
      (Physics|SetPhysicsLinearVelocity (Math|Vector|MakeVector (+ (.X (Math|Vector|BreakVector _returnvalue)) (Math|Random|RandomFloatinRange -1e+03 1e+03)) (* (.Y (Math|Vector|BreakVector _returnvalue_2)) -1.0) (.Z (Math|Vector|BreakVector _returnvalue_2))) false "None")
      (Audio|PlaySoundatLocation "/Game/Sounds/S_ballCollision.S_ballCollision" "0, 0, 0"))
    (:CastFailed
      ;[1 1 1] Enemy paddle collision detection section
      (bind _asbp_enemy_paddle (Utilities|Casting|CastToBP_Enemy_Paddle OtherActor)
        (:then
          (bind _returnvalue_3 (Physics|GetPhysicsLinearVelocity (Variables|/Game/Blueprints/BP_Enemy_Paddle.BP_Enemy_Paddle_C|GetStaticMesh _asbp_enemy_paddle) "None"))
          (bind _returnvalue_4 (Physics|GetPhysicsLinearVelocity "None"))
          (Physics|SetPhysicsLinearVelocity (Math|Vector|MakeVector (+ (.X (Math|Vector|BreakVector _returnvalue_3)) (Math|Random|RandomFloatinRange -1e+03 1e+03)) (* (.Y (Math|Vector|BreakVector _returnvalue_4)) -1.0) (.Z (Math|Vector|BreakVector _returnvalue_4))) false "None")
          (Audio|PlaySoundatLocation "/Game/Sounds/S_ballCollision.S_ballCollision" "0, 0, 0"))
        (:CastFailed
          ;[1 1 1] Player 2 Left Paddle Collision Detection
          (bind _asbp_paddle_left (Utilities|Casting|CastToBP_PaddleLeft OtherActor)
            (:then
              (Physics|GetPhysicsLinearVelocity _asbp_paddle_left "None")
              (bind _returnvalue_5 (Physics|GetPhysicsLinearVelocity "None"))
              (bind _returnvalue_6 (Physics|GetPhysicsLinearVelocity "None"))
              (Physics|SetPhysicsLinearVelocity (Math|Vector|MakeVector (+ (.X (Math|Vector|BreakVector _returnvalue_5)) (Math|Random|RandomFloatinRange -1e+03 1e+03)) (* (.Y (Math|Vector|BreakVector _returnvalue_6)) -1.0) (.Z (Math|Vector|BreakVector _returnvalue_6))) false "None")
              (Audio|PlaySoundatLocation "/Game/Sounds/S_ballCollision.S_ballCollision" "0, 0, 0"))
            (:CastFailed
              ;[1 1 1] Top and Bottom Boundary Collision Section
              (Utilities|Casting|CastToBlueprint_Horizontal_Boundary OtherActor
                (:then
                  (bind _returnvalue_7 (Physics|GetPhysicsLinearVelocity "None"))
                  (Physics|SetPhysicsLinearVelocity (Math|Vector|MakeVector (* (.X (Math|Vector|BreakVector _returnvalue_7)) -1.0) (.Y (Math|Vector|BreakVector _returnvalue_7)) (.Z (Math|Vector|BreakVector _returnvalue_7))) false "None")
                  (Audio|PlaySoundatLocation "/Game/Sounds/S_ballCollision.S_ballCollision" "0, 0, 0"))
                (:CastFailed
                  ;[1 1 1] Left Goal Collision Section
                  (Utilities|Casting|CastToBP_Left_Goal OtherActor
                    (:then
                      (Transformation|SetActorLocation "0, 0, 0" false)
                      (Audio|PlaySoundatLocation "/Game/Sounds/S_ballGoal.S_ballGoal" "0, 0, 0")
                      (Physics|SetPhysicsLinearVelocity "0,1500.000000, 0" false "None")
                      (Variables|Default|SetRPlayer_Score (+ (Variables|Default|GetRPlayer_Score) 1))
                      (bind _outactors (Actor|GetAllActorsOfClass "/Script/Engine.TextRenderActor"))
                      (for _array_element _outactors
                        (bind _astext_render_actor (Utilities|Casting|CastToTextRenderActor _array_element))
                        (if (Components|ComponentHasTag (Variables|/Script/Engine.TextRenderActor|GetTextRender _astext_render_actor) "RPlayerScoreTag")
                          (Rendering|Components|TextRender|SetText (Variables|/Script/Engine.TextRenderActor|GetTextRender _astext_render_actor) (Utilities|String|ToString(Integer) (Variables|Default|GetRPlayer_Score)))
                          (if (> (Variables|Default|GetRPlayer_Score) 11)
                            (Variables|Default|SetGameOver true)
                            (bind _outactors_2 (Actor|GetAllActorsOfClass "/Game/Blueprints/BP_PaddleLeft.BP_PaddleLeft_C"))
                            (if (> (Utilities|Array|Length _outactors_2) 0)
                              (Variables|Default|SetWinVariable "Player2 Wins!!!")
                              (else
                                (Variables|Default|SetWinVariable "Player Wins!!!")))))))
                    (:CastFailed
                      ;[1 1 1] Right Goal Collision Section
                      (Utilities|Casting|CastToBP_Right_Goal OtherActor)
                      (Transformation|SetActorLocation "0, 0, 0" false)
                      (Audio|PlaySoundatLocation "/Game/Sounds/S_ballGoal.S_ballGoal" "0, 0, 0")
                      (Physics|SetPhysicsLinearVelocity "0,-1500.000000, 0" false "None")
                      (Variables|Default|SetLPlayer_Score (+ (Variables|Default|GetLPlayer_Score) 1))
                      (bind _outactors_3 (Actor|GetAllActorsOfClass "/Script/Engine.TextRenderActor"))
                      (for _array_element_2 _outactors_3
                        (bind _astext_render_actor_2 (Utilities|Casting|CastToTextRenderActor _array_element_2))
                        (if (Components|ComponentHasTag (Variables|/Script/Engine.TextRenderActor|GetTextRender _astext_render_actor_2) "LPlayerScoreTag")
                          (Rendering|Components|TextRender|SetText (Variables|/Script/Engine.TextRenderActor|GetTextRender _astext_render_actor_2) (Utilities|String|ToString(Integer) (Variables|Default|GetLPlayer_Score)))
                          (if (> (Variables|Default|GetLPlayer_Score) 11)
                            (Variables|Default|SetGameOver true)
                            (bind _outactors_4 (Actor|GetAllActorsOfClass "/Game/Blueprints/BP_PaddleLeft.BP_PaddleLeft_C"))
                            (if (> (Utilities|Array|Length _outactors_4) 0)
                              (Variables|Default|SetWinVariable "Player1 Wins!!")
                              (else
                                (Variables|Default|SetWinVariable "AI Wins!!!")))))))))))))))))

(event EventTick
  (params (DeltaSeconds :type Float%20%28single-precision%29))
  (if (Variables|Default|GetGameOver)
    (Physics|SetPhysicsLinearVelocity "0, 0, 0" false "None")
    (bind _outactors (Actor|GetAllActorsOfClass "/Script/Engine.TextRenderActor"))
    (for _array_element _outactors
      (bind _aswin_text_blueprint (Utilities|Casting|CastToWin_Text_Blueprint _array_element))
      (Rendering|Components|TextRender|SetText _aswin_text_blueprint (Variables|Default|GetWinVariable))
      (Rendering|SetVisibility (Variables|/Script/Engine.TextRenderActor|GetTextRender _aswin_text_blueprint) true false)
      (Utilities|FlowControl|Delay 3.0)
      (Rendering|SetVisibility (Variables|/Script/Engine.TextRenderActor|GetTextRender _aswin_text_blueprint) false false)
      (bind _outactors_2 (Actor|GetAllActorsOfClass "/Game/Blueprints/BP_PaddleLeft.BP_PaddleLeft_C"))
      (if (> (Utilities|Array|Length _outactors_2) 0)
        (Game|OpenLevel(byName) "P2_Main")
        (else
          (Game|OpenLevel(byName) "P1_Main"))))))

(fn ConstructionScript)