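; AI opponent paddle that chases BP_Ball along the X axis using physics impulses.
; Each Tick it looks up all ball actors and, for each, applies an impulse from the clamped X offset to the ball, scaled by VariableAISpeed.
; If the paddle is past either symmetric X limit, it snaps back to that limit and zeroes its velocity instead of pushing.
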(event EventBeginPlay)

(event EventActorBeginOverlap
  (params (OtherActor :type Actor%20Object%20Reference)))

(event EventTick
  (params (DeltaSeconds :type Float%20%28single-precision%29))
  (bind _returnvalue (Transformation|GetActorLocation))
  (bind _returnvalue_2 (Transformation|GetActorLocation))
  (bind (_x _y _z) (Math|Vector|BreakVector _returnvalue))
  (bind (_x_2 _y_2 _z_2) (Math|Vector|BreakVector _returnvalue_2))
  (bind _outactors (Actor|GetAllActorsOfClass "/Game/Blueprints/BP_Ball.BP_Ball_C"))
  (for _array_element _outactors
    (bind _asbp_ball (Utilities|Casting|CastToBP_Ball _array_element))
    (if (> (.X (Math|Vector|BreakVector (Transformation|GetActorLocation))) 1.6e+03)
      (Transformation|SetActorLocation (Math|Vector|MakeVector 1.6e+03 _y_2 _z_2) false)
      (Physics|SetPhysicsLinearVelocity "0, 0, 0" false "None")
      (elif (< (.X (Math|Vector|BreakVector (Transformation|GetActorLocation))) -1.6e+03)
        (Transformation|SetActorLocation (Math|Vector|MakeVector -1.6e+03 _y _z) false)
        (Physics|SetPhysicsLinearVelocity "0, 0, 0" false "None")
        (else
          (Physics|AddImpulse (* (Math|Vector|MakeVector (Math|Float|Clamp(Float) (- (.X (Math|Vector|BreakVector (Transformation|GetActorLocation _asbp_ball))) (.X (Math|Vector|BreakVector (Transformation|GetActorLocation)))) -1e+01 1e+01) 0.0 0.0) (Variables|Default|GetVariable_AI_Speed)) "None" false))))))

(fn ConstructionScript)