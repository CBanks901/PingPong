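; BP_BallMenu is a physics ball, apparently for a menu scene, that bounces around between boundary actors.
; BeginPlay gives it a random velocity in the XY plane.
; On overlap, a horizontal boundary reverses its X velocity and a BP_Left_Goal, used for both side walls, reverses its Y velocity.
; Each bounce is scripted by setting physics velocity directly and plays a collision sound at world origin.
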(event EventBeginPlay
  (Physics|SetPhysicsLinearVelocity (Math|Vector|MakeVector (Math|Random|RandomFloatinRange -2e+03 2e+03) (Math|Random|RandomFloatinRange -1.5e+03 1.5e+03) 0.0) false "None"))

(event EventActorBeginOverlap
  (params (OtherActor :type Actor%20Object%20Reference))
  ;[1 1 1] Top and Bottom Boundary Collision Section
  (Utilities|Casting|CastToBlueprint_Horizontal_Boundary OtherActor
    (:then
      (bind _returnvalue (Physics|GetPhysicsLinearVelocity "None"))
      (Physics|SetPhysicsLinearVelocity (Math|Vector|MakeVector (* (.X (Math|Vector|BreakVector _returnvalue)) -1.0) (.Y (Math|Vector|BreakVector _returnvalue)) (.Z (Math|Vector|BreakVector _returnvalue))) false "None")
      (Audio|PlaySoundatLocation "/Game/Sounds/S_ballCollision.S_ballCollision" "0, 0, 0"))
    (:CastFailed
      ;[1 1 1] Wall collision using left goal for both sides
      (Utilities|Casting|CastToBP_Left_Goal OtherActor)
      (bind _returnvalue_2 (Physics|GetPhysicsLinearVelocity "None"))
      (Physics|SetPhysicsLinearVelocity (Math|Vector|MakeVector (.X (Math|Vector|BreakVector _returnvalue_2)) (* (.Y (Math|Vector|BreakVector _returnvalue_2)) -1.0) (.Z (Math|Vector|BreakVector _returnvalue_2))) false "None")
      (Audio|PlaySoundatLocation "/Game/Sounds/S_ballCollision.S_ballCollision" "0, 0, 0"))))

(fn ConstructionScript)